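; Base game mode for what appears to be a tile-based runner, handling level start and game over.
; On BeginPlay it shows the HUD widget and calls AddFloorTile ten times to lay the initial floor.
; Tick polls Health and, at zero or below, adds an end-game menu on every such frame, disables player input and quits after a short delay.
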(event EventTick
  (params (DeltaSeconds :type Float%20%28single-precision%29))
  ;[1 1 1] Show Start/End Game Widget
  (if (<= (Variables|Default|GetHealth) 0.0)
    (bind _returnvalue (UserInterface|CreateWidget "/Game/UI/BP_MenuEndGame.BP_MenuEndGame_C"))
    (UserInterface|Viewport|AddtoViewport _returnvalue 0)
    (Input|DisableInput (Game|GetPlayerCharacter 0) (Game|GetPlayerController 0))
    (Utilities|FlowControl|Delay 3.0)
    (Game|QuitGame 0 "Quit" false)))

(event EventBeginPlay
  ;[1 1 1] SpawnTile and Add HUD Widget
  (bind _returnvalue (UserInterface|CreateWidget "/Game/UI/BP_HUD.BP_HUD_C"))
  (UserInterface|Viewport|AddtoViewport _returnvalue 0)
  (for _index (range 0 9)
    (Class|TestTaskGameMode|AddFloorTile)))

(fn ConstructionScript)